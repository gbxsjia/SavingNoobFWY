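; CampManager is an AI Blueprint that shares alerts and enemy sightings among the agents of a camp.
; Agents register into a list, and CallSiren forwards an event location to every valid one within a given range of a start position.
; ReportEnemy records each enemy's last location and report time in a map.
; Query functions return that map, an enemy's last known location, or whether its report is still recent enough.
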(fn `CallSiren`
  (params (StartPostion :type "Vector Structure") (Range :type "Float (double-precision)") (EventLocation :type "Vector Structure"))
  (for _array_element (`self.AIAgents`)
    (`/Engine/EditorBlueprintResources/StandardMacros.IsValid` _array_element
      (:`Is Valid`
        (if (<= (`KismetMathLibrary.Vector_Distance` (`self.K2_GetActorLocation` _array_element) (`local.StartPostion`)) (`local.Range`))
          (`/Game/Blueprints/AI/AIController_Base.ReceiveReport` _array_element (`local.EventLocation`)))))))

(fn `GetEnemies`
  (returns (EnemyInfos :type "Map of Actor Object Reference to /Game/Blueprints/Misc/EnemyInfo Structure"))
  (return (`self.EnemyInfos`)))

(fn `GetEnemyLastLocation`
  (params (Enemy :type "Actor Object Reference"))
  (returns (valid :type Boolean) (loc :type "Vector Structure"))
  (bind (_value _returnvalue) (`BlueprintMapLibrary.Map_Find` (`self.EnemyInfos`) Enemy))
  (if _returnvalue
    (return true (`.LastLocation_5_0FC544FB4F85338F136E30A3E5B77155` (break `/Game/Blueprints/Misc/EnemyInfo` _value)))
    (else
      (return false (0.0 0.0 0.0)))))

(fn `IsEnemyTimeValid`
  (params (MaxTime :type "Float (double-precision)") (Enemy :type "Actor Object Reference"))
  (returns (result :type Boolean))
  (bind (_value _returnvalue) (`BlueprintMapLibrary.Map_Find` (`self.EnemyInfos`) Enemy))
  (if _returnvalue
    (return (<= (- (`KismetSystemLibrary.GetGameTimeInSeconds`) (`.LastReportTime_8_8466E84547C805BC3010FA8CB07242D4` (break `/Game/Blueprints/Misc/EnemyInfo` _value))) (`local.MaxTime`)))
    (else
      (return false))))

(fn `Regist AI`
  (params (NewItem :type "/Game/Blueprints/AI/AIController_Base Object Reference (by ref)"))
  (`KismetArrayLibrary.Array_Add` (`self.AIAgents`) NewItem))

(fn `ReportEnemy`
  (params (Enemy :type "Actor Object Reference"))
  (`BlueprintMapLibrary.Map_Add` (`self.EnemyInfos`) (`local.Enemy`) (make `/Game/Blueprints/Misc/EnemyInfo` (`self.K2_GetActorLocation` (`local.Enemy`)) (`KismetSystemLibrary.GetGameTimeInSeconds`))))

(fn `UserConstructionScript`)