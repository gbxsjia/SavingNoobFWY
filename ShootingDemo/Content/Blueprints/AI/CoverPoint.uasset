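; CoverPoint is an AI cover spot actor that a pawn can claim and that reports whether it shields against a given fire direction.
; Its construction script places ShootPlace, offset sideways for left or right high cover.
; EnterCover stores the owner and binds to its BPC_State death event, while CanEnter gates entry on a validity check.
; CanCover uses a forward-vector dot product; OwnerDead and ExitCover are empty, so nothing releases ownership here.
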(fn `CanCover`
  (params (ShootFromDirection :type "Vector Structure"))
  (returns (result :type Boolean))
  (return (< (`KismetMathLibrary.Dot_VectorVector` ShootFromDirection (`self.GetActorForwardVector`)) 0.0)))

(fn `CanEnter`
  (returns (result :type Boolean))
  (`/Engine/EditorBlueprintResources/StandardMacros.IsValid` null
    (:`Is Valid`
      (return false))
    (:`Is Not Valid`
      (return true))))

(fn `EnterCover`
  (params (Pawn :type "Actor Object Reference"))
  (if (!= Pawn (`self.OwnerPawn`))
    (bind _output_get (set `self.OwnerPawn` Pawn))
    (add `/Game/Blueprints/BPC_State.DeathEvent` (`self.GetComponentByClass` _output_get "/Game/Blueprints/BPC_State.BPC_State_C") (`|CreateDelegate` :!event `OwnerDead`))))

(fn `ExitCover`)

(fn `OwnerDead`
  (params (Damage :type "Float (double-precision)") (Instigator :type "Controller Object Reference") (Causer :type "Actor Object Reference")))

(fn `UserConstructionScript`
  (bind _offsetdistance (`self.offsetDistance`))
  (if (`self.isHighCover`)
    (`SceneComponent.K2_SetRelativeLocation` (`self.ShootPlace`) (select `bool` (`self.isLeft`) :`false` (`KismetMathLibrary.MakeVector` 0.0 _offsetdistance 92.0) :`true` (`KismetMathLibrary.MakeVector` 0.0 (* _offsetdistance -1.0) 92.0)) false false)
    (else
      (`SceneComponent.K2_SetRelativeLocation` (`self.ShootPlace`) (0.0 0.0 92.0) false false))))