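; CoverLib is a Blueprint function library whose FindCover function locates a usable CoverPoint around a position.
; It sphere-overlaps CoverPoint actors on a single object type channel within the given radius.
; Each point is tested in turn for whether it can be entered, covers against the shooting direction and can shoot the target.
; The first point passing all three checks is returned, with no distance or quality ranking.
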(fn `FindCover`
  (params (WorldContextObject :type "Object Object Reference") (SpherePos :type "Vector Structure") (SphereRadius :type "Float (double-precision)") (ShootFromDirectin :type "Vector Structure") (Target :type "Actor Object Reference"))
  (returns (cover :type "/Game/Blueprints/AI/CoverPoint Object Reference"))
  (bind _outactors (`KismetSystemLibrary.SphereOverlapActors` WorldContextObject SpherePos SphereRadius (`|MakeArray` "ObjectTypeQuery7" :!type "EObjectTypeQuery Enum") "/Game/Blueprints/AI/CoverPoint.CoverPoint_C"))
  (for _array_element _outactors
    (bind _ascover_point (cast `/Game/Blueprints/AI/CoverPoint` _array_element))
    (bind _result (`/Game/Blueprints/AI/CoverPoint.CanEnter` _ascover_point))
    (if _result
      (bind _result_2 (`/Game/Blueprints/AI/CoverPoint.CanCover` _ascover_point (`local.ShootFromDirectin`)))
      (if _result_2
        (bind _result_3 (`/Game/Blueprints/AI/CoverPoint.CanShootTarget` _ascover_point (`local.Target`)))
        (if _result_3
          (return _ascover_point)))))
  (return null))