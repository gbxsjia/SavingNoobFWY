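; Base AI controller that gives camp-based enemies stealth-style awareness across Normal, Alert and Battle states.
; On start it registers with its camp manager, runs the behavior tree, loads config into the Blackboard and arms the pawn.
; Sighted enemies raise an alert value by a distance curve, which decays after a state-dependent delay.
; State changes write events to the Blackboard; reports, sirens, retargeting and pawn death are also handled.
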(event `self.ReceiveBeginPlay`
  (`self.Initial`)
  (`BlackboardComponent.SetValueAsObject` (`self.Blackboard`) "Target" null)
  (`BlackboardComponent.SetValueAsVector` (`self.Blackboard`) "EventLocation" (-1000.0 -1000.0 90.0)))

(event `self.ReceiveTick`
  (params (DeltaSeconds :type "Float (single-precision)"))
  (if (`self.isAlive`)
    (`self.UpdateSightAlert`)))

(event `self.AIPerception.OnTargetPerceptionUpdated`
  (params (Actor :type "Actor Object Reference") (Stimulus :type "AIStimulus Structure"))
  (`self.UpdatePerception` Actor Stimulus))

(fn `AddAlertValue`
  (params (AlertValue :type "Float (double-precision)") (Source :type "Actor Object Reference"))
  (bind _source (`local.Source`))
  (bind _source_2 (`local.Source`))
  (bind _output_get (set `self.AlertValue` (+ AlertValue (`self.AlertValue`))))
  (if (>= _output_get 100.0)
    (`|ExecutionSequence`
      (:`then_0`
        (switch `/Game/Blueprints/Misc/AIState` (`self.AIState`)
          (:`NewEnumerator0`
            (`self.ChangeAlertState` "NewEnumerator1" 0.0 "NewEnumerator0" _source_2 (`self.K2_GetActorLocation` _source_2)))
          (:`NewEnumerator1`
            (`self.ChangeAlertState` "NewEnumerator2" 0.0 "NewEnumerator1" _source (`self.K2_GetActorLocation` _source)))
          (:`NewEnumerator2`
            (set `self.AlertValue` 100.0)))))))

(fn `CallSiren`
  (params (EventLocation :type "Vector Structure"))
  (bind _campmanager (`/Game/Blueprints/GI_Base.GetCampManager` (`self.GIBase`) (`self.Camp`)))
  (`/Game/Blueprints/AI/CampManager.CallSiren` _campmanager (`self.K2_GetActorLocation`) (`.SirenRange_21_857AEE564361C08DB3939690AA033E04` (break `/Game/Blueprints/Misc/AIInfo` (`self.AIInfo`))) EventLocation))

(fn `ChangeAlertState`
  (params (AIState :type "/Game/Blueprints/Misc/AIState Enum" :default "NewEnumerator0") (AlertValue :type "Float (double-precision)") (EnumValue :type "/Game/Blueprints/Misc/AIEventType Enum" :default "NewEnumerator3") (EventActor :type "Actor Object Reference") (EventLocation :type "Vector Structure"))
  (set `self.AIState` AIState)
  (set `self.AlertValue` AlertValue)
  (`BlackboardComponent.SetValueAsEnum` (`self.Blackboard`) "AIState" (`self.AIState`))
  (`BlackboardComponent.SetValueAsBool` (`self.Blackboard`) "ProcessingEvent" true)
  (`BlackboardComponent.SetValueAsEnum` (`self.Blackboard`) "EventType" EnumValue)
  (`BlackboardComponent.SetValueAsObject` (`self.Blackboard`) "Target" EventActor)
  (`BlackboardComponent.SetValueAsVector` (`self.Blackboard`) "EventLocation" EventLocation))

(fn `GetNearestEnemy`
  (returns (result :type "Actor Object Reference"))
  (locals (l_Result :type "Actor Object Reference") (l_Distance :type "Float (double-precision)" :default 9999999.0))
  (bind _campmanager (`/Game/Blueprints/GI_Base.GetCampManager` (`self.GIBase`) (`self.Camp`)))
  (bind _enemyinfos (`/Game/Blueprints/AI/CampManager.GetEnemies` _campmanager))
  (bind _keys (`BlueprintMapLibrary.Map_Keys` _enemyinfos))
  (for _array_element _keys
    (bind _returnvalue (`self.GetDistanceTo` _array_element (`self.MyPawn`)))
    (if (< _returnvalue (`local.l_Distance`))
      (set `local.l_Distance` _returnvalue)
      (set `local.l_Result` _array_element)))
  (return (`local.l_Result`)))

(fn `Initial`
  (bind ((`SirenRange_21_857AEE564361C08DB3939690AA033E04` _sirenrange) (`Weapon_16_75F024D14CCFD44A2FDC1595431E01A3` _weapon)) (break `/Game/Blueprints/Misc/AIInfo` (`self.AIInfo`)))
  (`|ExecutionSequence`
    (:`then_0`
      (bind _output_get (set `self.MyPawn` (`self.K2_GetPawn`)))
      (bind _camp (message `/Game/Blueprints/Misc/I_Camp.GetCamp` _output_get))
      (set `self.Camp` _camp)
      (bind _asgi_base (cast `/Game/Blueprints/GI_Base` (`GameplayStatics.GetGameInstance`)))
      (bind _output_get_2 (set `self.GIBase` _asgi_base))
      (bind _campmanager (`/Game/Blueprints/GI_Base.GetCampManager` _output_get_2 (`self.Camp`)))
      (`/Game/Blueprints/AI/CampManager.Regist AI` _campmanager self))
    (:`then_1`
      (`self.RunBehaviorTree` "/Game/Blueprints/AI/BT_Base.BT_Base"))
    (:`then_2`
      (bind _returnvalue (`|GetDataTableRow` (`self.AIConfigData`) "1")
        (:`then`
          (bind _output_get_3 (set `self.AIInfo` _returnvalue))
          (bind (_isbattleai _chaserange _cansearch _battlemode _cansiren) (break `/Game/Blueprints/Misc/AIInfo` _output_get_3))
          (`BlackboardComponent.SetValueAsBool` (`self.Blackboard`) "IsBattleAI" _isbattleai)
          (`BlackboardComponent.SetValueAsBool` (`self.Blackboard`) "CanSearch" _cansearch)
          (`BlackboardComponent.SetValueAsFloat` (`self.Blackboard`) "ChaseRange" _chaserange)
          (`BlackboardComponent.SetValueAsBool` (`self.Blackboard`) "CanSiren" _cansiren)
          (`BlackboardComponent.SetValueAsEnum` (`self.Blackboard`) "BattleMode" _battlemode))))
    (:`then_3`
      (bind _asals_anim_man_character_bp (cast `/Game/Blueprints/ALS_AnimMan_CharacterBP` (`self.MyPawn`)))
      (bind _returnvalue_2 (`|SpawnActorFromClass` _weapon (`KismetMathLibrary.MakeTransform` (0.0 0.0 0.0)) "Undefined" "OverrideRootScale" null null))
      (`/Game/Blueprints/ALS_AnimMan_CharacterBP.AddNewWeapon` _asals_anim_man_character_bp _returnvalue_2)
      (message `/Game/AdvancedLocomotionV4/Blueprints/Interfaces/ALS_Character_BPI.BPI_Set_OverlayState` _asals_anim_man_character_bp (defaults `Object` _weapon))
      (add `/Game/Blueprints/BPC_State.DeathEvent` (`/Game/Blueprints/ALS_AnimMan_CharacterBP.BPC_State` _asals_anim_man_character_bp) (`|CreateDelegate` :!event `OnPawnDeath`)))))

(fn `OnPawnDeath`
  (params (Damage :type "Float (double-precision)") (Instigator :type "Controller Object Reference") (Causer :type "Actor Object Reference"))
  (`self.UnPossess`)
  (set `self.isAlive` false)
  (`ActorComponent.K2_DestroyComponent` (`self.AIPerception`)))

(fn `ReceiveReport`
  (params (EventLocation :type "Vector Structure"))
  (if (`|EnumEquality` (`self.AIState`) "NewEnumerator0")
    (`self.ChangeAlertState` "NewEnumerator1" 50.0 "NewEnumerator6" null (`local.EventLocation`))))

(fn `ReduceAlertValue`
  (params (Amount :type "Float (double-precision)"))
  (bind _output_get (set `self.AlertValue` (- (`self.AlertValue`) Amount)))
  (if (<= _output_get 0.0)
    (`|ExecutionSequence`
      (:`then_0`
        (switch `/Game/Blueprints/Misc/AIState` (`self.AIState`)
          (:`NewEnumerator0`
            (set `self.AlertValue` 0.0))
          (:`NewEnumerator1`
            (`self.ChangeAlertState` "NewEnumerator0" 99.989998 "NewEnumerator4"))
          (:`NewEnumerator2`
            (`self.ChangeAlertState` "NewEnumerator2" 99.989998 "NewEnumerator5"))))
      (:`then_1`
        (`BlackboardComponent.SetValueAsEnum` (`self.Blackboard`) "AIState" (`self.AIState`))))))

(fn `ResetBattleTarget`
  (locals (l_InvalidTargets :type "Array of Actor Object Reference") (l_Target :type "Actor Object Reference") (l_Range :type "Float (double-precision)" :default 9999999.0) (l_OldTarget :type "Actor Object Reference"))
  (bind _l_oldtarget (`local.l_OldTarget`))
  (`|ExecutionSequence`
    (:`then_0`
      (bind _asactor (cast `Actor` (`BlackboardComponent.GetValueAsObject` (`self.Blackboard`) "Target")))
      (set `local.l_OldTarget` _asactor))
    (:`then_1`
      (for _array_element (`self.EnemiesInSight`)
        (bind _alive (message `/Game/Blueprints/Misc/I_Damagable.IsAlive` _array_element))
        (if (not _alive)
          (`KismetArrayLibrary.Array_Add` (`local.l_InvalidTargets`) _array_element)))
      (for _array_element_2 (`local.l_InvalidTargets`)
        (`KismetArrayLibrary.Array_RemoveItem` (`self.EnemiesInSight`) _array_element_2))
      (for _array_element_3 (`self.EnemiesInSight`)
        (bind _returnvalue (`self.GetDistanceTo` _array_element_3 (`self.MyPawn`)))
        (if (<= _returnvalue (`local.l_Range`))
          (set `local.l_Target` _array_element_3)
          (set `local.l_Range` _returnvalue)))
      (bind _l_target (`local.l_Target`)
        (:`then`
          (`BlackboardComponent.SetValueAsObject` (`self.Blackboard`) "Target" _l_target :!label _label))
        (:`else`
          (bind _alive_2 (message `/Game/Blueprints/Misc/I_Damagable.IsAlive` _l_oldtarget))
          (if _alive_2
            (goto _label)
            (else
              (`self.ChangeAlertState` "NewEnumerator1" 99.0 "NewEnumerator5" null (`self.K2_GetActorLocation` _l_oldtarget)))))))))

(fn `SendEvent`
  (params (EnumValue :type "/Game/Blueprints/Misc/AIEventType Enum" :default "NewEnumerator3")))

(fn `UpdatePerception`
  (params (Actor :type "Actor Object Reference") (AIStimulus :type "AIStimulus Structure (by ref)"))
  (bind (_age _expirationage _strength _stimuluslocation _receiverlocation _tag _bsuccessfullysensed) (break `AIStimulus` AIStimulus))
  ;[1 1 1] 是不是友军
  (bind _camp (message `/Game/Blueprints/Misc/I_Camp.GetCamp` Actor))
  (if (!= _camp (`self.Camp`))
    ;[1 1 1] 是不是视觉
    (if (== _tag "None")
      (if _bsuccessfullysensed
        (`KismetArrayLibrary.Array_Add` (`self.EnemiesInSight`) (`local.Actor`))
        (else
          (`KismetArrayLibrary.Array_RemoveItem` (`self.EnemiesInSight`) (`local.Actor`)))))))

(fn `UpdateSightAlert`
  (`|ExecutionSequence`
    (:`then_0`
      (for _array_element (`self.EnemiesInSight`)
        (`self.AddAlertValue` (* (`CurveFloat.GetFloatValue` (`self.SightAlertCurve`) (`self.GetDistanceTo` _array_element (`self.MyPawn`))) (`GameplayStatics.GetWorldDeltaSeconds`)) _array_element)))
    (:`then_1`
      (if (> (`KismetArrayLibrary.Array_Length` (`self.EnemiesInSight`)) 0)
        (set `self.LastSenseTime` (`KismetSystemLibrary.GetGameTimeInSeconds`))
        (elif (>= (- (`KismetSystemLibrary.GetGameTimeInSeconds`) (`self.LastSenseTime`)) (select `/Game/Blueprints/Misc/AIState` (`self.AIState`) :`NewEnumerator0` 4.0 :`NewEnumerator1` 15.0 :`NewEnumerator2` 30.0 :!type "Float (single-precision)"))
          (`self.ReduceAlertValue` (* (`GameplayStatics.GetWorldDeltaSeconds`) 20.0)))))))

(fn `UserConstructionScript`)