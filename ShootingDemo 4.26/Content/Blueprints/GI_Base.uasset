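; GI_Base is a base game instance that provides access to the CampManager for a given camp.
; GetCampManager looks up the camp in the CampManagers map and returns the stored manager if present.
; Otherwise it spawns a CampManager actor with that camp, caches it in the map and returns it, so managers are created lazily, one per camp.
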(fn `GetCampManager`
  (params (Camp :type Integer))
  (returns (campManager :type "/Game/Blueprints/AI/CampManager Object Reference"))
  (if (`BlueprintMapLibrary.Map_Contains` (`self.CampManagers`) Camp)
    (return (`BlueprintMapLibrary.Map_Find` (`self.CampManagers`) (`local.Camp`)))
    (else
      (bind _returnvalue (`|SpawnActorFromClass` "/Game/Blueprints/AI/CampManager.CampManager_C" (`KismetMathLibrary.MakeTransform` (0.0 0.0 0.0)) "Undefined" "OverrideRootScale" null (`local.Camp`) null))
      (`BlueprintMapLibrary.Map_Add` (`self.CampManagers`) (`local.Camp`) _returnvalue)
      (return _returnvalue))))